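; BP_Bird is a bird actor that repeatedly flies along its spline, with a separate visual component placed at a chosen spline key.
; StartFlying waits, runs a timeline that moves Bird along the spline, then restarts itself after a random pause.
; A timeline event track triggers a second timeline that animates the visual's opacity through a dynamic material.
; AttachToPlayer snaps the actor relative to the player pawn, with yaw turned 180 degrees.
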(event `self.ReceiveBeginPlay`
  (bind _visluals (`self.Visluals`))
  (bind _returnvalue (`PrimitiveComponent.CreateDynamicMaterialInstance` _visluals 0 (`PrimitiveComponent.GetMaterial` _visluals 0) "None"))
  (bind _output_get (set `self.VisualsMaterial` _returnvalue))
  (`PrimitiveComponent.SetMaterial` (`self.Visluals`) 0 _output_get))

(event `AttachToPlayer`
  (`self.K2_SetActorLocation` (+ (`SplineComponent.GetLocationAtSplineInputKey` (`self.Spline`) (`self.SplineKeyForVisuals`) "Local") (`self.K2_GetActorLocation` (`GameplayStatics.GetPlayerPawn` 0))) false true)
  (`self.K2_SetActorRotation` (`KismetMathLibrary.MakeRotator` (.roll (`self.K2_GetActorRotation` (`GameplayStatics.GetPlayerPawn` 0))) (.pitch (`self.K2_GetActorRotation` (`GameplayStatics.GetPlayerPawn` 0))) (- (.yaw (`self.K2_GetActorRotation` (`GameplayStatics.GetPlayerPawn` 0))) 180.0))))

(event `StartFlying`
  (bind _spline (`self.Spline`))
  (`KismetSystemLibrary.Delay` (`self.TimeBeforeFlyStart`))
  (bind (_direction _alpha) (`Timeline|FlyingTimeline` :!via `PlayFromStart`)
    (:`Update`
      (`SceneComponent.K2_SetWorldLocation` (`self.Bird`) (`SplineComponent.GetLocationAtDistanceAlongSpline` (`self.Spline`) (`KismetMathLibrary.Lerp` 0.0 (`SplineComponent.GetDistanceAlongSplineAtSplinePoint` _spline (- (`SplineComponent.GetNumberOfSplinePoints` _spline) 1)) _alpha) "World") false true))
    (:`Finished`
      (`KismetSystemLibrary.Delay` (`KismetMathLibrary.RandomFloatInRange` 3.0 5.0))
      (`self.StartFlying`))
    (:`SpawnVisuals`
      (bind (_direction_2 _opacity) (`Timeline|Visuals Timeline` :!via `PlayFromStart`)
        (:`Update`
          (`MaterialInstanceDynamic.SetScalarParameterValue` (`self.VisualsMaterial`) "OpacityMultiplier" _opacity))))))

(event `self.ReceiveTick`
  (params (DeltaSeconds :type "Float (single-precision)"))
  (set `self.Delta Seconds` DeltaSeconds)
  (`self.Tick`))

(fn `UserConstructionScript`
  (`SceneComponent.K2_SetRelativeLocation` (`self.Visluals`) (`SplineComponent.GetLocationAtSplineInputKey` (`self.Spline`) (`self.SplineKeyForVisuals`) "Local") false false))