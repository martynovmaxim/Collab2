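; BP_Window is a breakable window actor that shatters once when its Destroy event fires.
; It hides the intact glass mesh and reveals the shard static meshes parented under the Scene component.
; Each shard becomes a simulated, physics-only Destructible body, pushed outward by a radial impulse from the RadialForce component's location.
; A DoOnce gate keeps the break from repeating.
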(event `Destroy`
  (`/Engine/EditorBlueprintResources/StandardMacros.DoOnce` false
    (:`Completed`
      (`SceneComponent.SetVisibility` (`self.FullGlass`) false false)
      (for _array_element (`SceneComponent.GetChildrenComponents` (`self.Scene`) false)
        (bind _asstatic_mesh_component (cast `StaticMeshComponent` _array_element))
        (`PrimitiveComponent.SetCollisionObjectType` _asstatic_mesh_component "ECC_Destructible")
        (`PrimitiveComponent.SetCollisionEnabled` _asstatic_mesh_component "PhysicsOnly")
        (`SceneComponent.SetVisibility` _asstatic_mesh_component true false)
        (`PrimitiveComponent.SetSimulatePhysics` _asstatic_mesh_component true)
        (`PrimitiveComponent.AddRadialImpulse` _asstatic_mesh_component (`SceneComponent.K2_GetComponentLocation` (`self.RadialForce`)) 200.0 1000.0 "RIF_Linear" true)))))

(fn `UserConstructionScript`)