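; BP_AudioManager plays music tracks with crossfading between two audio components.
; Play fades out the active component over a fifth of the fade duration while the other fades in with the new sound, then Switch swaps their roles.
; With nothing active, Play starts on Music1 and sets Music2 as standby.
; Stop halts or briefly fades the active component, then clears it.
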(event `Play`
  (params (NewSound :type "SoundCue Object Reference") (FadeDuration :type "Float (double-precision)"))
  (bind _music1 (`self.Music1`))
  (bind _inactivecomponent (`self.InActiveComponent`))
  (`self.ActiveComponent`
    (:`then`
      (`AudioComponent.FadeOut` (`self.ActiveComponent`) (/ FadeDuration 5.0) 0.0 "Linear")
      (`AudioComponent.SetSound` _inactivecomponent NewSound)
      (`AudioComponent.FadeIn` _inactivecomponent FadeDuration 1.0 0.0 "Linear")
      (`self.Switch`))
    (:`else`
      (`AudioComponent.SetSound` _music1 NewSound)
      (bind _output_get (set `self.ActiveComponent` _music1))
      (`AudioComponent.FadeIn` _output_get FadeDuration 1.0 0.0 "Linear")
      (set `self.InActiveComponent` (`self.Music2`)))))

(event `Stop`
  (params (Instant :type Boolean))
  (bind _activecomponent (`self.ActiveComponent`))
  (if Instant
    (`AudioComponent.Stop` _activecomponent)
    (else
      (`AudioComponent.FadeOut` _activecomponent 0.5 0.0 "Linear")))
  (set `self.ActiveComponent` null))

(fn `Switch`
  (locals (Tmp :type "AudioComponent Object Reference"))
  (bind _output_get (set `local.Tmp` (`self.ActiveComponent`)))
  (set `self.ActiveComponent` (`self.InActiveComponent`))
  (set `self.InActiveComponent` _output_get))

(fn `UserConstructionScript`)