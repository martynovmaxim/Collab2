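; BP_PuzzlePrevTrigger is a sphere trigger that fails the puzzle when the player pawn re-enters it.
; It arms itself by setting Active when the pawn first leaves the sphere, so a later begin overlap calls FailPuzzle on the referenced Player.
; The construction script sizes the sphere from that Player's SplineMeshDistance when the reference is valid.
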(event `self.Sphere.OnComponentBeginOverlap`
  (params (OverlappedComponent :type "PrimitiveComponent Object Reference") (OtherActor :type "Actor Object Reference") (OtherComp :type "PrimitiveComponent Object Reference") (OtherBodyIndex :type Integer) (bFromSweep :type Boolean) (SweepResult :type "HitResult Structure (by ref)"))
  (if (== OtherActor (`GameplayStatics.GetPlayerPawn` 0))
    (if (`self.Active`)
      (`/Game/Core/RollingBP/BP_Ball.FailPuzzle` (`self.Player`)))))

(event `self.Sphere.OnComponentEndOverlap`
  (params (OverlappedComponent :type "PrimitiveComponent Object Reference") (OtherActor :type "Actor Object Reference") (OtherComp :type "PrimitiveComponent Object Reference") (OtherBodyIndex :type Integer))
  (if (== OtherActor (`GameplayStatics.GetPlayerPawn` 0))
    (set `self.Active` true)))

(fn `UserConstructionScript`
  (bind _player (`self.Player`)
    (:`then`
      (`SphereComponent.SetSphereRadius` (`self.Sphere`) (`/Game/Core/RollingBP/BP_Ball.SplineMeshDistance` _player) false))
    (:`else`)))