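; BP_Photo is a ball puzzle, started on trigger overlap, that points the player's gravity into its plane.
; The construction script builds spline meshes along every spline, mapped per spline; Tick reveals the segment nearest the ball.
; Four collectible overlaps crack, then remove, the exit glass.
; Leaving the trigger ends the puzzle if all are collected, otherwise an active puzzle resets the ball, trail and points with a camera shake.
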(event `FailPuzzle`
  (bind _exit_glass (`self.Exit_Glass`))
  (bind _player (`self.Player`))
  (bind _returnvalue (`SceneComponent.K2_GetComponentLocation` (`self.Start`)))
  (if (`self.Active`)
    (bind _keys (`BlueprintMapLibrary.Map_Keys` (`self.SplineMeshes`)))
    (for _array_element _keys
      (for _array_element_2 (`.Meshes_6_81D9525C457F09F10574D1865F9592D7` (break `/Game/Core/Puzzle/S_SplineMesh` (`BlueprintMapLibrary.Map_Find` (`self.SplineMeshes`) _array_element)))
        (`SceneComponent.SetVisibility` _array_element_2 false false)))
    (`PrimitiveComponent.SetAllPhysicsLinearVelocity` (`/Game/Core/RollingBP/BP_Ball.Sphere` _player) (0.0 0.0 0.0) false)
    (`self.K2_SetActorLocation` _player _returnvalue false false)
    (`GameplayStatics.PlayWorldCameraShake` "/Game/Core/Puzzle/BP_PuzzleFailShake.BP_PuzzleFailShake_C" _returnvalue 50000.0)
    (`SceneComponent.SetVisibility` (`self.Point`) true false)
    (`SceneComponent.SetVisibility` (`self.Point1`) true false)
    (`SceneComponent.SetVisibility` (`self.Point2`) true false)
    (`SceneComponent.SetVisibility` (`self.Point3`) true false)
    (set `self.NumberOfCopllectedPoints` 0)
    (`SceneComponent.SetVisibility` _exit_glass false false)
    (`PrimitiveComponent.SetCollisionEnabled` _exit_glass "NoCollision")
    (`PrimitiveComponent.SetMaterial` (`self.Exit_Glass`) 0 "/Game/MaterialLibrary/M_Orzelek_Assets/Materials/Free/Glass/M_Glass_Clean.M_Glass_Clean")))

(event `EndPuzzle`
  (if (>= (`self.NumberOfCopllectedPoints`) 4)
    (`/Game/Core/RollingBP/BP_Ball.EndPuzzle` (`self.Player`))
    (`self.SetActorTickEnabled` false)
    (else
      (`self.FailPuzzle`))))

(event `Start Puzzle`
  (bind _asbp_ball (cast `/Game/Core/RollingBP/BP_Ball` (`GameplayStatics.GetPlayerPawn` 0)))
  (bind _output_get (set `self.Player` _asbp_ball))
  (`/Game/Core/RollingBP/BP_Ball.StartPuzzle` _output_get self)
  (`SceneComponent.K2_AttachToComponent` (`self.PlayerPos`) (`Actor.RootComponent` _asbp_ball) "None" "KeepRelative" "KeepRelative" "KeepRelative" true)
  (`self.SetActorTickEnabled` true)
  (set `/Game/Core/RollingBP/BP_Ball.GravityDirection` (`KismetMathLibrary.Normal` (`KismetMathLibrary.NegateVector` (`SceneComponent.GetUpVector` (`self.Plane`)))) (`self.Player`))
  (`KismetSystemLibrary.Delay` 3.0)
  (set `self.Active` true))

(event `self.ReceiveTick`
  (params (DeltaSeconds :type "Float (single-precision)"))
  (bind _returnvalue (`SceneComponent.K2_GetComponentLocation` (`self.PlayerPos`)))
  (set `self.SmallestDistance` 500.0)
  (bind _keys (`BlueprintMapLibrary.Map_Keys` (`self.SplineMeshes`)))
  (for _array_element _keys
    (bind _returnvalue_2 (`SplineComponent.FindInputKeyClosestToWorldLocation` _array_element _returnvalue))
    (bind _returnvalue_3 (`KismetMathLibrary.VSize` (- _returnvalue (`SplineComponent.GetLocationAtSplineInputKey` _array_element _returnvalue_2 "World"))))
    (if (< _returnvalue_3 (`self.SmallestDistance`))
      (set `self.SmallestDistance` _returnvalue_3)
      (set `self.ClosestMesh` (`|GetArrayItem` (`.Meshes_6_81D9525C457F09F10574D1865F9592D7` (break `/Game/Core/Puzzle/S_SplineMesh` (`BlueprintMapLibrary.Map_Find` (`self.SplineMeshes`) _array_element))) (`KismetMathLibrary.FTrunc` _returnvalue_2)))))
  (`SceneComponent.SetVisibility` (`self.ClosestMesh`) true false))

(event `self.MainTrigger.OnComponentBeginOverlap`
  (params (OverlappedComponent :type "PrimitiveComponent Object Reference") (OtherActor :type "Actor Object Reference") (OtherComp :type "PrimitiveComponent Object Reference") (OtherBodyIndex :type Integer) (bFromSweep :type Boolean) (SweepResult :type "HitResult Structure (by ref)"))
  (`self.Start Puzzle`))

(event `self.MainTrigger.OnComponentEndOverlap`
  (params (OverlappedComponent :type "PrimitiveComponent Object Reference") (OtherActor :type "Actor Object Reference") (OtherComp :type "PrimitiveComponent Object Reference") (OtherBodyIndex :type Integer))
  (`self.EndPuzzle`))

(event `self.Sphere.OnComponentBeginOverlap`
  (params (OverlappedComponent :type "PrimitiveComponent Object Reference") (OtherActor :type "Actor Object Reference") (OtherComp :type "PrimitiveComponent Object Reference") (OtherBodyIndex :type Integer) (bFromSweep :type Boolean) (SweepResult :type "HitResult Structure (by ref)"))
  (`SceneComponent.SetVisibility` OverlappedComponent false true)
  (`self.IncreaseNumberOfCollecetedPoints`))

(event `self.Sphere1.OnComponentBeginOverlap`
  (params (OverlappedComponent :type "PrimitiveComponent Object Reference") (OtherActor :type "Actor Object Reference") (OtherComp :type "PrimitiveComponent Object Reference") (OtherBodyIndex :type Integer) (bFromSweep :type Boolean) (SweepResult :type "HitResult Structure (by ref)"))
  (`SceneComponent.SetVisibility` OverlappedComponent false true)
  (`self.IncreaseNumberOfCollecetedPoints`))

(event `self.Sphere2.OnComponentBeginOverlap`
  (params (OverlappedComponent :type "PrimitiveComponent Object Reference") (OtherActor :type "Actor Object Reference") (OtherComp :type "PrimitiveComponent Object Reference") (OtherBodyIndex :type Integer) (bFromSweep :type Boolean) (SweepResult :type "HitResult Structure (by ref)"))
  (`SceneComponent.SetVisibility` OverlappedComponent false true)
  (`self.IncreaseNumberOfCollecetedPoints`))

(event `self.Sphere3.OnComponentBeginOverlap`
  (params (OverlappedComponent :type "PrimitiveComponent Object Reference") (OtherActor :type "Actor Object Reference") (OtherComp :type "PrimitiveComponent Object Reference") (OtherBodyIndex :type Integer) (bFromSweep :type Boolean) (SweepResult :type "HitResult Structure (by ref)"))
  (`SceneComponent.SetVisibility` OverlappedComponent false true)
  (`self.IncreaseNumberOfCollecetedPoints`))

(event `self.Spline.OnComponentBeginOverlap`
  (params (OverlappedComponent :type "PrimitiveComponent Object Reference") (OtherActor :type "Actor Object Reference") (OtherComp :type "PrimitiveComponent Object Reference") (OtherBodyIndex :type Integer) (bFromSweep :type Boolean) (SweepResult :type "HitResult Structure (by ref)")))

(event `IncreaseNumberOfCollecetedPoints`
  (bind _exit_glass (`self.Exit_Glass`))
  (bind _result (`/Engine/EditorBlueprintResources/StandardMacros.IncrementInt` (`self.NumberOfCopllectedPoints`))
    (:`  `
      (if (>= _result 1)
        (`PrimitiveComponent.SetMaterial` (`self.Exit_Glass`) 0 "/Game/MaterialLibrary/M_Orzelek_Assets/Materials/Free/Glass/M_GlassShattered_1.M_GlassShattered_1")
        (if (>= (`self.NumberOfCopllectedPoints`) 4)
          (`SceneComponent.SetVisibility` _exit_glass false false)
          (`PrimitiveComponent.SetCollisionEnabled` _exit_glass "NoCollision"))))))

(fn `UserConstructionScript`
  (locals (CurrentSplineMesh :type "SplineMeshComponent Object Reference") (ActiveSpline :type "SplineComponent Object Reference") (CurrentSplineMeshes :type "Array of SplineMeshComponent Object Reference"))
  (bind _glass (`self.Glass`))
  (bind _activespline (`local.ActiveSpline`))
  (`|ExecutionSequence`
    (:`then_0`
      (`SceneComponent.SetVisibility` _glass (`SceneComponent.bVisible` _glass) true))
    (:`then_1`
      (for _array_element (`self.K2_GetComponentsByClass` "/Script/Engine.SplineComponent")
        (set `local.ActiveSpline` _array_element)
        (for _index (range (+ (- (`SplineComponent.GetNumberOfSplinePoints` (`local.ActiveSpline`)) -2) 1))
          (bind _returnvalue (`AddComponent|NODE_AddSplineMeshComponent-0` :`RelativeTransform` (`SceneComponent.GetRelativeTransform` (`local.ActiveSpline`))))
          (bind _output_get (set `local.CurrentSplineMesh` _returnvalue))
          (`KismetArrayLibrary.Array_Add` (`local.CurrentSplineMeshes`) _output_get)
          (bind _returnvalue_2 (+ _index 1))
          (`SplineMeshComponent.SetStartAndEnd` (`local.CurrentSplineMesh`) (`SplineComponent.GetLocationAtSplinePoint` _activespline _index "Local") (`SplineComponent.GetTangentAtSplinePoint` _activespline _index "Local") (`SplineComponent.GetLocationAtSplinePoint` _activespline _returnvalue_2 "Local") (`SplineComponent.GetTangentAtSplinePoint` _activespline _returnvalue_2 "Local") true))
        (`BlueprintMapLibrary.Map_Add` (`self.SplineMeshes`) (`local.ActiveSpline`) (make `/Game/Core/Puzzle/S_SplineMesh` (`local.CurrentSplineMeshes`)))
        (`KismetArrayLibrary.Array_Clear` (`local.CurrentSplineMeshes`))))))