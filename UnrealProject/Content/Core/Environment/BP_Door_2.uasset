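; BP_Door_2 is a door that starts open and swings shut when a BP_Ball overlaps its Box trigger.
; It swaps visibility between three components: DoorOpened, a DoorMoving stand-in that a timeline rotates to zero relative rotation, and DoorClosed.
; When the swing finishes, it also hides the Plane and disables the Box collision, so the door stays closed.
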(event `self.ReceiveBeginPlay`
  (`SceneComponent.SetVisibility` (`self.DoorOpened`) true true)
  (`SceneComponent.SetVisibility` (`self.Plane`) true true)
  (`SceneComponent.SetVisibility` (`self.DoorClosed`) false true)
  (`SceneComponent.SetVisibility` (`self.DoorMoving`) false true))

(event `Close Door`
  (set `self.StartRotation` (`SceneComponent.RelativeRotation` (`self.DoorMoving`)))
  (`SceneComponent.SetVisibility` (`self.DoorMoving`) true true)
  (`SceneComponent.SetVisibility` (`self.DoorOpened`) false true)
  (bind (_direction _newtrack_0) (`Timeline|DoorRotation` :!via `PlayFromStart`)
    (:`Update`
      (`SceneComponent.K2_SetRelativeRotation` (`self.DoorMoving`) (`KismetMathLibrary.RLerp` (`self.StartRotation`) (struct) _newtrack_0 true) false false))
    (:`Finished`
      (`SceneComponent.SetVisibility` (`self.DoorMoving`) false true)
      (`SceneComponent.SetVisibility` (`self.Plane`) false true)
      (`SceneComponent.SetVisibility` (`self.DoorClosed`) true true)
      (`PrimitiveComponent.SetCollisionEnabled` (`self.Box`) "NoCollision"))))

(event `self.Box.OnComponentBeginOverlap`
  (params (OverlappedComponent :type "PrimitiveComponent Object Reference") (OtherActor :type "Actor Object Reference") (OtherComp :type "PrimitiveComponent Object Reference") (OtherBodyIndex :type Integer) (bFromSweep :type Boolean) (SweepResult :type "HitResult Structure (by ref)"))
  (cast `/Game/Core/RollingBP/BP_Ball` OtherActor)
  (`self.Close Door`))

(fn `UserConstructionScript`)