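; BP_Door is a door actor that plays a two-stage opening animation when its OpenDoor event is called.
; A HandleRotation timeline turns the handle's relative rotation, then on finish a DoorRotation timeline swings the root's world rotation.
; Both stages lerp along the shortest path from the captured rotation to hard-coded targets, so the open yaw is absolute in world space.
; It has no closing logic, and a delayed self-open is left unconnected.
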(event `self.ReceiveBeginPlay`)

(event `Open Door`
  (set `self.StartRotation` (`SceneComponent.RelativeRotation` (`self.Handle`)))
  (bind (_direction _newtrack_0) (`Timeline|HandleRotation`)
    (:`Update`
      (`SceneComponent.K2_SetRelativeRotation` (`self.Handle`) (`KismetMathLibrary.RLerp` (`self.StartRotation`) (struct :`Pitch` -30.0 :`Yaw` 90.0) _newtrack_0 true) false false))
    (:`Finished`
      (set `self.StartRotation` (`SceneComponent.K2_GetComponentRotation` (`self.DefaultSceneRoot`)))
      (bind (_direction_2 _newtrack_0_2) (`Timeline|DoorRotation`)
        (:`Update`
          (`SceneComponent.K2_SetWorldRotation` (`self.DefaultSceneRoot`) (`KismetMathLibrary.RLerp` (`self.StartRotation`) (struct :`Yaw` 255.0) _newtrack_0_2 true) false false))))))

(fn `UserConstructionScript`)