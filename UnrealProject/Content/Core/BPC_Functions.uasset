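; A Blueprint helper collection of small utility functions for vectors, actor queries and arrays.
; GetVectorAxis keeps selected axes of a vector and zeroes the rest, while AddToArray returns an array with an element added.
; GetClosestActor finds the nearest actor in line of sight of an origin via debug-drawn Visibility traces.
; It seeds the search with the first array entry, which is returned even if occluded when nothing visible is closer.
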(fn `addToArray`
  (params (input :type "Array of SplineMeshComponent Object Reference") (add :type "SplineMeshComponent Object Reference"))
  (returns (Result :type "Array of SplineMeshComponent Object Reference"))
  (locals (NewLocalVar_0 :type "Array of SplineMeshComponent Object Reference"))
  (bind _output_get (set `local.NewLocalVar_0` input))
  (`KismetArrayLibrary.Array_Add` _output_get add)
  (return (`local.NewLocalVar_0`)))

(fn `GetClosestActor`
  (params (Actors :type "Array of /Game/Core/Gum/BP_GumPoint Object Reference") (Origin :type "Actor Object Reference"))
  (returns (ClosestActor :type "Actor Object Reference") (DistanceToClosestActor :type "Float (double-precision)"))
  (locals (Closest :type "Actor Object Reference") (DistanceToClosest :type "Float (double-precision)"))
  (bind _origin (`local.Origin`))
  (bind _output_get (set `local.Closest` (`|GetArrayItem` Actors)))
  (set `local.DistanceToClosest` (`Actor.GetDistanceTo` _output_get Origin))
  (for _array_element (`local.Actors`)
    (`/Engine/EditorBlueprintResources/StandardMacros.IsValid` _array_element
      (:`Is Valid`
        (bind _outhit (`KismetSystemLibrary.LineTraceSingle` (`local.__WorldContext`) (`Actor.K2_GetActorLocation` _origin) (`Actor.K2_GetActorLocation` _array_element) "TraceTypeQuery1" false (`|MakeArray` _origin) "ForOneFrame" false (struct :`R` 1.0 :`A` 1.0) (struct :`G` 1.0 :`A` 1.0) 0.0))
        (if (== (`.HitActor` (`GameplayStatics.BreakHitResult` _outhit)) _array_element)
          (bind _returnvalue (`Actor.GetDistanceTo` _array_element (`local.Origin`)))
          (if (< _returnvalue (`local.DistanceToClosest`))
            (set `local.Closest` _array_element)
            (set `local.DistanceToClosest` _returnvalue))))))
  (return (`local.Closest`) (`local.DistanceToClosest`)))

(fn `GetVectorAxis`
  (params (InVector :type "Vector Structure") (X :type Boolean) (Y :type Boolean) (Z :type Boolean))
  (returns (OutVector :type "Vector Structure"))
  (bind (_invector_x _invector_y _invector_z) (`KismetMathLibrary.BreakVector` (`local.InVector`)))
  (return (`KismetMathLibrary.MakeVector` (`KismetMathLibrary.SelectFloat` _invector_x 0.0 X) (`KismetMathLibrary.SelectFloat` _invector_y 0.0 Y) (`KismetMathLibrary.SelectFloat` _invector_z 0.0 Z))))