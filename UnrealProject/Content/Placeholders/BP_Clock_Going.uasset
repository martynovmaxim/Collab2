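; Placeholder clock actor that keeps its pendulum swinging from BeginPlay.
; A looping one-second timer restarts a timeline that lerps the Pendulum's roll away from its cached starting rotation.
; An unconnected chain would stop the timer, rotate the ArrowDynamic hand, then play a smaller pendulum swing, but it never runs.
; A swing-count comparison is also left unused.
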(event `self.ReceiveBeginPlay`
  (bind _pendulumstartrotation (`self.PendulumStartRotation`))
  (set `self.PendulumStartRotation` (`SceneComponent.RelativeRotation` (`self.Pendulum`)))
  (set `self.ArrowStartRotation` (`SceneComponent.RelativeRotation` (`self.ArrowDynamic`)))
  (bind _returnvalue (`KismetSystemLibrary.K2_SetTimerDelegate` (delegate `PendulumSwing`) 1.0 true))
  (set `self.SwingTimer` _returnvalue)
  (bind (_direction _newtrack_0) (`Timeline|PendulumSwingLoop` :!label _label)
    (:`Update`
      (`SceneComponent.K2_SetRelativeRotation` (`self.Pendulum`) (`KismetMathLibrary.RLerp` _pendulumstartrotation (`KismetMathLibrary.MakeRotator` (+ (.roll _pendulumstartrotation) 20.0)) _newtrack_0 true) false false))))

(event `PendulumSwing`
  (goto _label :!via `PlayFromStart`))

(fn `UserConstructionScript`)