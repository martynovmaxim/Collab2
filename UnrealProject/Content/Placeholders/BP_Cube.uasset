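; Placeholder cube actor that gives itself a random color.
; The construction script creates a dynamic material instance from the Cube component's first material, assigns it to slot 0 and stores it in a Material variable.
; It then sets the Color vector parameter to random red, green and blue values, so the color re-rolls each time construction runs.
; The event graph has no active logic.
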(fn `UserConstructionScript`
  (bind _returnvalue (`KismetMaterialLibrary.CreateDynamicMaterialInstance` (`|GetArrayItem` (`MeshComponent.GetMaterials` (`self.Cube`)))))
  (bind _output_get (set `self.Material` _returnvalue))
  (`PrimitiveComponent.SetMaterial` (`self.Cube`) 0 _output_get)
  (`MaterialInstanceDynamic.SetVectorParameterValue` (`self.Material`) "Color" (`KismetMathLibrary.MakeColor` (`KismetMathLibrary.RandomFloatInRange` 0.0 1.0) (`KismetMathLibrary.RandomFloatInRange` 0.0 1.0) (`KismetMathLibrary.RandomFloatInRange` 0.0 1.0))))