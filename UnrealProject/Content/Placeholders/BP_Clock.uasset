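; Clock actor that animates a swinging pendulum and, after a set number of swings, moves its dynamic hand.
; A looping one-second timer replays the pendulum timeline, which lerps roll from the starting rotation and increments a swing counter on finish.
; Once the counter exceeds its maximum, the timer is cleared and chained timelines rotate the hand toward zero rotation, then play a smaller pendulum swing.
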(event `self.ReceiveBeginPlay`
  (bind _pendulumstartrotation (`self.PendulumStartRotation`))
  (set `self.PendulumStartRotation` (`SceneComponent.RelativeRotation` (`self.Pendulum`)))
  (set `self.ArrowStartRotation` (`SceneComponent.RelativeRotation` (`self.ArrowDynamic`)))
  (bind _returnvalue (`KismetSystemLibrary.K2_SetTimerDelegate` (delegate `PendulumSwing`) 1.0 true))
  (set `self.SwingTimer` _returnvalue)
  (bind (_direction _newtrack_0) (`Timeline|PendulumSwingLoop` :!label _label)
    (:`Update`
      (`SceneComponent.K2_SetRelativeRotation` (`self.Pendulum`) (`KismetMathLibrary.RLerp` _pendulumstartrotation (`KismetMathLibrary.MakeRotator` (+ (.roll _pendulumstartrotation) 20.0)) _newtrack_0 true) false false))
    (:`Finished`
      (`/Engine/EditorBlueprintResources/StandardMacros.IncrementInt` (`self.PendulumSwingsNumber`)))))

(event `PendulumSwing`
  (bind _pendulumstartrotation (`self.PendulumStartRotation`))
  (if (<= (`self.PendulumSwingsNumber`) (`self.PendulumSwingsMaxNumber`))
    (goto _label :!via `PlayFromStart`)
    (else
      (`KismetSystemLibrary.K2_ClearAndInvalidateTimerHandle` (`self.SwingTimer`))
      (bind (_direction _newtrack_0) (`Timeline|Timeline_1` :!via `PlayFromStart`)
        (:`Update`
          (`SceneComponent.K2_SetRelativeRotation` (`self.ArrowDynamic`) (`KismetMathLibrary.RLerp` (`self.ArrowStartRotation`) (struct) _newtrack_0 true) false false))
        (:`Finished`
          (bind (_direction_2 _newtrack_0_2) (`Timeline|Timeline_0` :!via `PlayFromStart`)
            (:`Update`
              (`SceneComponent.K2_SetRelativeRotation` (`self.Pendulum`) (`KismetMathLibrary.RLerp` _pendulumstartrotation (`KismetMathLibrary.MakeRotator` (+ (.roll _pendulumstartrotation) 10.0)) _newtrack_0_2 true) false false))))))))

(fn `UserConstructionScript`)